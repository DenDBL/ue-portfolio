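; Access validator actor that signals granted or denied access with a colored light and swings a door open on success.
; BeginPlay binds handlers to the OnAccessGranted and OnAccessDenied dispatchers, which this graph never calls itself.
; Denial shows red briefly; a grant shows green and plays a timeline rotating the door 90 degrees.
; A retriggerable delay on timeline updates turns the light off and reverses the door after a pause.
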(event Custom|OnAccessGranted_Event
  (bind _light (Variables|Default|GetLight))
  (Rendering|Components|Light|SetLightColor _light "(R=0.000000,G=1.000000,B=0.023097,A=1.000000)" false)
  (Rendering|Components|Light|SetIntensity _light 5e+03)
  (bind _anglealpha (Timeline|TL_DoorOpen PlayFromStart)
    (:Update
      (Transformation|SetRelativeRotation (Variables|Default|GetDoor) (Math|Rotator|Lerp(Rotator) "0, 0, 0" "0,90.000000, 0" _anglealpha true) false false)
      (Utilities|FlowControl|RetriggerableDelay 1e+01)
      (Rendering|Components|Light|SetIntensity (Variables|Default|GetLight) 0.0)
      (Timeline|TL_DoorOpen Reverse))))

(event Custom|OnAccessDenied_Event
  (bind _light (Variables|Default|GetLight))
  (Rendering|Components|Light|SetLightColor _light "(R=1.000000,G=0.000000,B=0.082829,A=1.000000)" false)
  (Rendering|Components|Light|SetIntensity _light 5e+03)
  (Utilities|FlowControl|RetriggerableDelay 5.0)
  (Rendering|Components|Light|SetIntensity (Variables|Default|GetLight) 0.0))

(event EventBeginPlay
  (EventDispatchers|AssignOnAccessGranted (delegate Custom|OnAccessGranted_Event))
  (EventDispatchers|BindEventtoOnAccessDenied (delegate Custom|OnAccessDenied_Event)))

(event Collision|EventActorBeginOverlap
  (params (OtherActor :type Actor%20Object%20Reference)))

(event EventTick
  (params (DeltaSeconds :type Float%20%28single-precision%29)))

(fn ConstructionScript)