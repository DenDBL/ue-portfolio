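; BP_ProtoValve is a prototype interactable valve actor that the player turns by dragging the mouse horizontally.
; Trigger start and stop events set and clear the Freezed flag on the triggering BP_ProtoChar.
; The drag event adds world yaw to the whole actor from BP_ProtoController's left/right axis value, with no clamping.
; RotateValve is an empty stub.
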(event EventBeginPlay
  (Input|EnableInput 0))

(event Collision|EventActorBeginOverlap
  (params (OtherActor :type Actor%20Object%20Reference)))

(event EventTick
  (params (DeltaSeconds :type Float%20%28single-precision%29)))

(event EventTriggerItem
  (params (Actor :type Actor%20Object%20Reference))
  (Variables|/Game/Core/ProtoBP/BP_ProtoChar.BP_ProtoChar_C|Setfreezed (.AsBP%20Proto%20Char (Utilities|Casting|CastToBP_ProtoChar Actor)) true))

(event EventTriggerItemStop
  (params (Actor :type Actor%20Object%20Reference))
  (Variables|/Game/Core/ProtoBP/BP_ProtoChar.BP_ProtoChar_C|Setfreezed (.AsBP%20Proto%20Char (Utilities|Casting|CastToBP_ProtoChar Actor)) false))

(event EventHandleMouseXDrag
  (params (Actor :type Actor%20Object%20Reference))
  (Class|Actor|AddActorWorldRotation (Math|Rotator|MakeRotator 0.0 0.0 (Variables|/Game/Core/ProtoBP/BP_ProtoController.BP_ProtoController_C|GetAxis%20Value%20LeftRight (.AsBP%20Proto%20Controller (Utilities|Casting|CastToBP_ProtoController (Game|GetPlayerController 0)))))))

(fn ConstructionScript)

(fn RotateValve
  (if true
    _))