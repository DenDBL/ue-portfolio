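; Player controller for the prototype character that routes player input to the possessed BP_ProtoChar.
; On BeginPlay it casts and caches the controlled pawn as PossessedChar.
; Axis inputs forward movement and look values to the character, with the horizontal look value also stored in AxisValueLeftRight.
; Action inputs call the character's item pickup, two-slot selection, and press/release item use functions.
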(event EventBeginPlay
  (bind _asbp_proto_char (Utilities|Casting|CastToBP_ProtoChar (Pawn|GetControlledPawn)))
  (Variables|Default|SetPossessedChar _asbp_proto_char))

(event EventTick
  (params (DeltaSeconds :type Float%20%28single-precision%29)))

(event Input|ActionEvents|InputActionPickUp
  (params (Key :type Key%20Structure :default "None"))
  (:Pressed
    (Default|PickUpItem (Variables|Default|GetPossessedChar))))

(event Input|ActionEvents|InputActionChoose1Slot
  (params (Key :type Key%20Structure :default "None"))
  (:Pressed
    (Default|ChooseSlot (Variables|Default|GetPossessedChar))))

(event Input|ActionEvents|InputActionChoose2Slot
  (params (Key :type Key%20Structure :default "None"))
  (:Pressed
    (Default|ChooseSlot (Variables|Default|GetPossessedChar) 1)))

(event Input|ActionEvents|InputActionTrigger
  (params (Key :type Key%20Structure :default "None"))
  (bind _possessedchar (Variables|Default|GetPossessedChar))
  (:Pressed
    (Default|UseItem _possessedchar))
  (:Released
    (Default|StopUsingItem _possessedchar)))

(event Input|AxisEvents|InputAxisLookLeft/Right
  (params (AxisValue :type Float%20%28single-precision%29))
  (Default|LookLeftRight (Variables|Default|GetPossessedChar) AxisValue)
  (Variables|Default|SetAxis%20Value%20LeftRight AxisValue))

(event Input|AxisEvents|InputAxisMoveRight/Left
  (params (AxisValue :type Float%20%28single-precision%29))
  (Default|MoveLeftRight (Variables|Default|GetPossessedChar) AxisValue))

(event Input|AxisEvents|InputAxisLookUp/Down
  (params (AxisValue :type Float%20%28single-precision%29))
  (Default|LookUpDown (Variables|Default|GetPossessedChar) AxisValue))

(event Input|AxisEvents|InputAxisMoveForward/Backward
  (params (AxisValue :type Float%20%28single-precision%29))
  (Default|MoveForwardBackward (Variables|Default|GetPossessedChar) AxisValue))

(fn ConstructionScript)