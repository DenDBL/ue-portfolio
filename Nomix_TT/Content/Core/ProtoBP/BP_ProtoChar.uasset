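; BP_ProtoChar is a prototype first-person-style character that moves, looks around and interacts with items.
; Pickup and use line-trace from the camera out to the sphere's radius, then send interface-style messages to the hit actor.
; The sphere tracks nearby actors and stops item triggers when they leave.
; Freezed blocks movement and pitch, redirecting horizontal mouse input to the looked-at object as drag, while slot selection goes to InventoryComponent.
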(event OnComponentBeginOverlap(Sphere)
  (params (OverlappedComponent :type Primitive%20Component%20Object%20Reference) (OtherActor :type Actor%20Object%20Reference) (OtherComp :type Primitive%20Component%20Object%20Reference) (OtherBodyIndex :type Integer) (bFromSweep :type Boolean) (SweepResult :type Hit%20Result%20Structure%20%28by%20ref%29))
  (Utilities|Array|AddUnique (Variables|Default|GetobjectsInRadius) OtherActor))

(event OnComponentEndOverlap(Sphere)
  (params (OverlappedComponent :type Primitive%20Component%20Object%20Reference) (OtherActor :type Actor%20Object%20Reference) (OtherComp :type Primitive%20Component%20Object%20Reference) (OtherBodyIndex :type Integer))
  (Utilities|Array|RemoveItem (Variables|Default|GetobjectsInRadius) OtherActor)
  (Class|BIItems|TriggerItemStop(Message) OtherActor self))

(event EventBeginPlay)

(event Collision|EventActorBeginOverlap
  (params (OtherActor :type Actor%20Object%20Reference)))

(event EventTick
  (params (DeltaSeconds :type Float%20%28single-precision%29)))

(fn ConstructionScript)

(fn MoveForwardBackward
  (params (Value :type Float%20%28double-precision%29))
  (if (not (Variables|Default|Getfreezed))
    (Pawn|Input|AddMovementInput (Math|Vector|GetForwardVector (Variables|Default|GetCamera)) Value false)))

(fn MoveLeftRight
  (params (Value :type Float%20%28double-precision%29))
  (if (not (Variables|Default|Getfreezed))
    (Pawn|Input|AddMovementInput (Math|Vector|GetRightVector (Variables|Default|GetCamera)) Value false)))

(fn LookUpDown
  (params (Value :type Float%20%28double-precision%29))
  (if (not (Variables|Default|Getfreezed))
    (Pawn|Input|AddControllerPitchInput Value)))

(fn LookLeftRight
  (params (Value :type Float%20%28double-precision%29))
  (bind _lookedat (Variables|Default|GetLookedAt))
  (if (not (Variables|Default|Getfreezed))
    (Pawn|Input|AddControllerYawInput Value)
    (else
      (Utilities|IsValid _lookedat
        (:Is%20Valid
          (Class|BIItems|HandleMouseXDrag(Message) _lookedat self))))))

(fn GetLookingatObject
  (bind _camera (Variables|Default|GetCamera))
  (bind _returnvalue (Transformation|GetWorldLocation _camera))
  (bind _outhit (Collision|LineTraceByChannel _returnvalue (+ _returnvalue (* (Math|Vector|GetForwardVector _camera) (Math|Conversions|ToVector(Float) (Variables|/Script/Engine.SphereComponent|GetSphereRadius (Variables|Default|GetSphere))))) "TraceTypeQuery3" false 0 "None"))
  (return (.HitActor (Collision|BreakHitResult _outhit))))

(fn PickUpItem
  (bind _actor (CallFunction|GetLookingatObject))
  (bind _output_get (Variables|Default|SetLookedAt _actor))
  (Utilities|IsValid _output_get
    (:Is%20Valid
      (Class|BIItems|PickUp(Message) _output_get self))))

(fn ChooseSlot
  (params (Slot%20Number :type Integer))
  (Default|SelectItem (Variables|Default|GetInventoryComponent) Slot%20Number))

(fn UseItem
  (bind _actor (CallFunction|GetLookingatObject))
  (bind _output_get (Variables|Default|SetLookedAt _actor))
  (bind _output_get_2 (Variables|Default|SetobjectInAction _output_get))
  (Class|BIItems|TriggerItem(Message) _output_get_2 self))

(fn StopUsingItem
  (Class|BIItems|TriggerItemStop(Message) (Variables|Default|GetobjectInAction) self))