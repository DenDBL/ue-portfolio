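; Actor component that gives its owner a fixed-size slot inventory of prototype card actors, with one selected slot.
; It sizes the slot array on BeginPlay and places each added item in the first empty slot, ignoring it when full.
; Adding or selecting refreshes every stored card, so only the selected one is visible with query-only box collision while the rest are hidden without collision.
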(event EventBeginPlay
  (CallFunction|InitInventoryComponent))

(event EventTick
  (params (DeltaSeconds :type Float%20%28single-precision%29)))

(fn InitInventoryComponent
  (CallFunction|InitSlots))

(fn InitSlots
  (if (!= (Variables|Default|GetslotsCount) 0)
    (for _index (range 0 (- (Variables|Default|GetslotsCount) 1))
      (Utilities|Array|Add (Variables|Default|Getslots) 0))))

(fn AddItemtoInventory
  (params (Item :type Actor%20Object%20Reference))
  (bind _index (Utilities|FlowControl|ForLoopwithBreak 0 (- (Variables|Default|GetslotsCount) 1) :!label _label)
    (:LoopBody
      (if (not (Utilities|IsValid (Utilities|Array|Get(acopy) (Variables|Default|Getslots) _index)))
        (Utilities|Array|SetArrayElem (Variables|Default|Getslots) _index Item)
        (CallFunction|UpdateSelectedItem)
        (goto _label Break)))))

(fn UpdateSelectedItem
  (bind _slots (Variables|Default|Getslots))
  (bind _selectedslot (Variables|Default|GetselectedSlot))
  (bind _output (Utilities|Array|Get(acopy) _slots _selectedslot))
  (bind _asbp_proto_card (Utilities|Casting|CastToBP_ProtoCard _output))
  (for _array_element (Variables|Default|Getslots)
    (Utilities|IsValid _array_element
      (:Is%20Valid
        (Rendering|SetActorHiddenInGame (.AsBP%20Proto%20Card (Utilities|Casting|CastToBP_ProtoCard _array_element)) true)
        (Collision|SetCollisionEnabled (Variables|/Game/Core/ProtoBP/BP_ProtoCard.BP_ProtoCard_C|GetBox (.AsBP%20Proto%20Card (Utilities|Casting|CastToBP_ProtoCard _array_element))) "NoCollision"))))
  (Utilities|IsValid _output
    (:Is%20Valid
      (Rendering|SetActorHiddenInGame _asbp_proto_card false)
      (Collision|SetCollisionEnabled (Variables|/Game/Core/ProtoBP/BP_ProtoCard.BP_ProtoCard_C|GetBox _asbp_proto_card) "QueryOnly"))))

(fn SelectItem
  (params (Slot :type Integer))
  (Variables|Default|SetselectedSlot Slot)
  (CallFunction|UpdateSelectedItem))

(fn GetSelectedItem
  (return (Utilities|Array|Get(acopy) (Variables|Default|Getslots) (Variables|Default|GetselectedSlot))))