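; Debug actor that shows X/Y index labels on walkable tiles of every BP_Grid when tile index display is enabled.
; It binds to each grid's tile data updates, and toggling the display either refreshes every tile or clears all labels.
; TextRenderActors are spawned on demand, cached in a map keyed by index and grid, and destroyed for missing or unwalkable tiles.
; Tick yaws every label to face opposite the BP_Pawn's rotation.
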(event EventBeginPlay
  (bind _outactors (Actor|GetAllActorsOfClass "/Game/BP/Core/Grid/BP_Grid.BP_Grid_C"))
  (for _array_element _outactors
    (EventDispatchers|BindEventtoOnTileDataUpdate _array_element (EventDispatchers|CreateEvent :!event UpdateTextonTile))))

(event Collision|EventActorBeginOverlap
  (params (OtherActor :type Actor%20Object%20Reference)))

(event EventTick
  (params (DeltaSeconds :type Float%20%28single-precision%29))
  (bind _returnvalue (Actor|GetActorOfClass "/Game/BP/Core/Player/BP_Pawn.BP_Pawn_C"))
  (bind _values (Utilities|Map|Values (Variables|Default|GetspawnedTexts)))
  (for _array_element _values
    (Transformation|SetActorRotation _array_element (Math|Rotator|MakeRotator 0.0 0.0 (+ (.yaw (Transformation|GetActorRotation _returnvalue)) 1.8e+02)))))

(fn ConstructionScript)

(fn GetTextActor
  (params (index :type Int%20Point%20Structure) (grid :type BP%20Grid%20Object%20Reference))
  (bind _output_get (LocalVariables|SetActor (.Value (Utilities|Map|Find (Variables|Default|GetspawnedTexts) (Utilities|Struct|MakeS_IndexAndGrid index grid)))))
  (Utilities|IsValid _output_get
    (:Is%20Valid
      (return (LocalVariables|GetActor)))
    (:Is%20Not%20Valid
      (bind _returnvalue (Game|SpawnActorfromClass "/Script/Engine.TextRenderActor" (Math|Transform|MakeTransform "0, 0, 0" "0, 0, 0" "1.000000,1.000000,1.000000") "AlwaysSpawn" 0 0))
      (bind _output_get_2 (LocalVariables|SetActor _returnvalue))
      (Utilities|Map|Add (Variables|Default|GetspawnedTexts) (Utilities|Struct|MakeS_IndexAndGrid index grid) _output_get_2)
      (Actor|Tick|SetActorTickEnabled (LocalVariables|GetActor))
      (Collision|SetActorEnableCollision (LocalVariables|GetActor) false)
      (Rendering|Components|TextRender|SetHorizontalAlignment (Variables|/Script/Engine.TextRenderActor|GetTextRender (LocalVariables|GetActor)) "EHTA_Center")
      (Class|TextRenderComponent|SetVerticalAlignment (Variables|/Script/Engine.TextRenderActor|GetTextRender (LocalVariables|GetActor)) "EVRTA_TextCenter")
      (return (LocalVariables|GetActor)))))

(fn DestroyTextActor
  (params (Index :type Int%20Point%20Structure) (grid :type BP%20Grid%20Object%20Reference))
  (bind _output_get (LocalVariables|Setactor (.Value (Utilities|Map|Find (Variables|Default|GetspawnedTexts) (Utilities|Struct|MakeS_IndexAndGrid Index grid)))))
  (Utilities|IsValid _output_get
    (:Is%20Valid
      (Actor|DestroyActor (LocalVariables|Getactor))
      (Utilities|Map|Remove (Variables|Default|GetspawnedTexts) (Utilities|Struct|MakeS_IndexAndGrid Index grid)))))

(fn ClearAllTextValues
  (bind _values (Utilities|Map|Values (Variables|Default|GetspawnedTexts)))
  (for _array_element _values
    (Actor|DestroyActor _array_element))
  (Utilities|Map|Clear (Variables|Default|GetspawnedTexts)))

(fn UpdateTextonTile
  (params (index :type Int%20Point%20Structure) (grid :type BP%20Grid%20Object%20Reference))
  (bind _gridtiles (Variables|/Game/BP/Core/Grid/BP_Grid.BP_Grid_C|GetgridTiles grid))
  (bind (_value _returnvalue) (Utilities|Map|Find _gridtiles index))
  (if (Variables|Default|GetShow%20Tiles%20Indexes)
    (if _returnvalue
      (bind _output_get (LocalVariables|Setdata _value))
      (if (CallFunction|IsTileTypeWalkable (.type _output_get))
        (bind _text_render_actor (CallFunction|GetTextActor index grid))
        (LocalVariables|SettextActor _text_render_actor)
        (LocalVariables|SetText (Utilities|String|Append (Utilities|String|ToString(Integer) (.x index)) " " (Utilities|String|ToString(Integer) (.y index))))
        (Rendering|Components|TextRender|SetText (Variables|/Script/Engine.TextRenderActor|GetTextRender (LocalVariables|GettextActor)) (Utilities|Text|ToText(String) (LocalVariables|GetText)))
        (bind _returnvalue_2 (Actor|GetActorOfClass "/Game/BP/Core/Player/BP_Pawn.BP_Pawn_C"))
        (Transformation|SetActorTransform (LocalVariables|GettextActor) (Math|Transform|MakeTransform (+ (.location (.transform (LocalVariables|Getdata))) "0,0,10.000000") (Math|Rotator|MakeRotator 0.0 0.0 (+ (.yaw (Transformation|GetActorRotation _returnvalue_2)) 1.8e+02)) "1.000000,1.000000,1.000000"))
        (Rendering|Components|TextRender|SetTextRenderColor (Variables|/Script/Engine.TextRenderActor|GetTextRender (LocalVariables|GettextActor)) (Math|Color|MakeColor 0 0 0 1))
        (else
          (CallFunction|DestroyTextActor index grid :!label _label)))
      (else
        (goto _label)))))

(fn ShowTileIndexes
  (params (Show%20Tiles :type Boolean))
  (bind _output_get (Variables|Default|SetShow%20Tiles%20Indexes Show%20Tiles))
  (if _output_get
    (bind _outactors (Actor|GetAllActorsOfClass "/Game/BP/Core/Grid/BP_Grid.BP_Grid_C"))
    (for _array_element _outactors
      (bind _keys (Utilities|Map|Keys (Variables|/Game/BP/Core/Grid/BP_Grid.BP_Grid_C|GetgridTiles _array_element)))
      (for _array_element_2 _keys
        (CallFunction|UpdateTextonTile _array_element_2 _array_element)))
    (else
      (CallFunction|ClearAllTextValues))))