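; Utility actor that renders grid cells as instanced static meshes, highlighting each by its state.
; An index array parallel to the instances maps grid indices to instance slots, so re-adding a cell replaces its old instance.
; The highest-priority state (Selected, Hovered, IsNeighbour, PartOfPath) sets color and fill, written to per-instance custom data for the material.
; Initialization supplies mesh, material, base color and collision; actor tick is disabled.
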(event EventBeginPlay)

(event Collision|EventActorBeginOverlap
  (params (OtherActor :type Actor%20Object%20Reference)))

(fn ConstructionScript
  (Actor|Tick|SetActorTickEnabled false))

(fn AddInstance
  (params (InstanceTransform :type Transform%20%28by%20ref%29) (index :type Int%20Point%20Structure%20%28by%20ref%29) (states :type Array%20of%20E_TileState%20Enums :default "NewEnumerator0"))
  (CallFunction|RemoveInstance index)
  (Components|InstancedStaticMesh|AddInstance (Variables|Default|GetInstancedStaticMesh) InstanceTransform true)
  (bind _returnvalue (Utilities|Array|Add (Variables|Default|GetinstanceIndexes) index))
  (LocalVariables|SetI _returnvalue)
  (bind (_color _fill) (CallFunction|GetColorfromStates states))
  (Components|InstancedStaticMesh|SetCustomDataValue (Variables|Default|GetInstancedStaticMesh) (LocalVariables|GetI) 0 (.R (Utilities|Struct|BreakLinearColor _color)) false)
  (Components|InstancedStaticMesh|SetCustomDataValue (Variables|Default|GetInstancedStaticMesh) (LocalVariables|GetI) 1 (.G (Utilities|Struct|BreakLinearColor _color)) false)
  (Components|InstancedStaticMesh|SetCustomDataValue (Variables|Default|GetInstancedStaticMesh) (LocalVariables|GetI) 2 (.B (Utilities|Struct|BreakLinearColor _color)) false)
  (Components|InstancedStaticMesh|SetCustomDataValue (Variables|Default|GetInstancedStaticMesh) (LocalVariables|GetI) 3 _fill false))

(fn RemoveInstance
  (params (index :type Int%20Point%20Structure%20%28by%20ref%29))
  (if (Utilities|Array|ContainsItem (Variables|Default|GetinstanceIndexes) index)
    (Class|InstancedStaticMeshComponent|RemoveInstance (Variables|Default|GetInstancedStaticMesh) (Utilities|Array|FindItem (Variables|Default|GetinstanceIndexes) index))
    (Utilities|Array|RemoveItem (Variables|Default|GetinstanceIndexes) index)))

(fn ClearInstances
  (Components|InstancedStaticMesh|ClearInstances (Variables|Default|GetInstancedStaticMesh))
  (Utilities|Array|Clear (Variables|Default|GetinstanceIndexes)))

(fn InitGridMeshInst
  (params (collision :type ECollisionEnabled%20Enum :default "NoCollision") (Mesh :type Static%20Mesh%20Object%20Reference) (Material :type Material%20Interface%20Object%20Reference) (color :type Linear%20Color%20Structure))
  (Components|StaticMesh|SetStaticMesh (Variables|Default|GetInstancedStaticMesh) Mesh)
  (Rendering|Material|SetMaterial (Variables|Default|GetInstancedStaticMesh) 0 Material)
  (Rendering|Material|SetVectorParameterValueonMaterials (Variables|Default|GetInstancedStaticMesh) "color" (Math|Conversions|ToVector(LinearColor) color))
  (Collision|SetCollisionEnabled (Variables|Default|GetInstancedStaticMesh) collision))

(fn GetColorfromStates
  (params (States :type Array%20of%20E_TileState%20Enums :default "NewEnumerator0"))
  (if (== (Utilities|Array|Length States) 0)
    (return "" 0.0)
    (else
      (for _array_element (Utilities|Array|MakeArray "NewEnumerator2" "NewEnumerator1" "NewEnumerator3" "NewEnumerator4")
        (if (Utilities|Array|ContainsItem States _array_element)
          (return (Utilities|Select :Index _array_element :NewEnumerator0 "" :NewEnumerator1 "(R=0.500000,G=0.970503,B=1.000000,A=1.000000)" :NewEnumerator2 "(R=1.000000,G=0.000000,B=0.018721,A=1.000000)" :NewEnumerator3 "(R=0.946717,G=1.000000,B=0.380143,A=1.000000)" :NewEnumerator4 "(R=0.017549,G=0.885417,B=0.000000,A=1.000000)") 1.0)))
      (return "" 0.0))))