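; Simple grid-bound character that walks tile paths within and between BP_Grids, with hover highlight and selection arrow.
; A sphere trace finds its grid and tile at construction and BeginPlay, when it also snaps to that tile.
; Timelines step through path indexes, lerping location and look-at rotation while switching animation state.
; Multi-grid paths chain segments by teleporting through the BP_GridTransition matching the current tile, then resuming movement.
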(event Custom|MoveThroughPath_Event
  (params (pathIndexes :type Array%20of%20Int%20Point%20Structures))
  (if (> (Utilities|Array|Length pathIndexes) 0)
    (CallFunction|SetAnimation "NewEnumerator1")
    (bind _output_get (Variables|Default|SetPath%20Indexes pathIndexes))
    (Variables|Default|SetcurrentTransform (Transformation|GetActorTransform) :!label _label)
    (Variables|Default|SettargetTransform (.transform (.Value (Utilities|Map|Find (Variables|/Game/BP/Core/Grid/BP_Grid.BP_Grid_C|GetgridTiles (Variables|Default|Getgrid)) (Utilities|Array|Get(acopy) _output_get)))))
    (Variables|Default|SettargetTransform (Math|Transform|MakeTransform (.location (Variables|Default|GettargetTransform)) (Math|Rotator|FindLookatRotation (.location (Variables|Default|GetcurrentTransform)) (.location (Variables|Default|GettargetTransform))) "1.000000,1.000000,1.000000"))
    (Components|Timeline|SetPlayRate (Variables|Default|GetmovementOnGrid) (Variables|Default|GetSpeed))
    (bind (_direction _time_alpha _rotationalpha) (Timeline|movementOnGrid PlayFromStart)
      (:Update
        (Transformation|SetActorLocation (Math|Vector|Lerp(Vector) (.location (Variables|Default|GetcurrentTransform)) (.location (Variables|Default|GettargetTransform)) _time_alpha) false false)
        (Transformation|SetActorRotation (Math|Rotator|Lerp(Rotator) (.rotation (Variables|Default|GetcurrentTransform)) (.rotation (Variables|Default|GettargetTransform)) _rotationalpha true)))
      (:Finished
        (Variables|Default|SettileIndex (Utilities|Array|Get(acopy) (Variables|Default|GetPath%20Indexes)))
        (Utilities|Array|RemoveIndex (Variables|Default|GetPath%20Indexes))
        (if (> (Utilities|Array|Length (Variables|Default|GetPath%20Indexes)) 0)
          (goto _label)
          (else
            (CallFunction|SetAnimation "NewEnumerator0")))))))

(event Custom|MoveThroughPathBetweenGrids_Event
  (params (PathBetweenGrids :type Array%20of%20S%20Indexes%20and%20Grid%20Structures))
  (if (> (Utilities|Array|Length PathBetweenGrids) 0)
    (CallFunction|SetAnimation "NewEnumerator1")
    (Variables|Default|SetPath%20Between%20Grids PathBetweenGrids)
    (Variables|Default|SetPath%20Indexes (.index (Utilities|Array|Get(acopy) (Variables|Default|GetPath%20Between%20Grids))))
    (if (> (Utilities|Array|Length (Variables|Default|GetPath%20Indexes)) 0)
      (Variables|Default|SetcurrentTransform (Transformation|GetActorTransform) :!label _label)
      (Variables|Default|SettargetTransform (.transform (.Value (Utilities|Map|Find (Variables|/Game/BP/Core/Grid/BP_Grid.BP_Grid_C|GetgridTiles (Variables|Default|Getgrid)) (Utilities|Array|Get(acopy) (Variables|Default|GetPath%20Indexes))))))
      (Variables|Default|SettargetTransform (Math|Transform|MakeTransform (.location (Variables|Default|GettargetTransform)) (Math|Rotator|FindLookatRotation (.location (Variables|Default|GetcurrentTransform)) (.location (Variables|Default|GettargetTransform))) "1.000000,1.000000,1.000000"))
      (Components|Timeline|SetPlayRate (Variables|Default|GetmovementOnGrids) (Variables|Default|GetSpeed))
      (bind (_direction _time_alpha _rotationalpha) (Timeline|movementOnGrids PlayFromStart)
        (:Update
          (Transformation|SetActorLocation (Math|Vector|Lerp(Vector) (.location (Variables|Default|GetcurrentTransform)) (.location (Variables|Default|GettargetTransform)) _time_alpha) false false)
          (Transformation|SetActorRotation (Math|Rotator|Lerp(Rotator) (.rotation (Variables|Default|GetcurrentTransform)) (.rotation (Variables|Default|GettargetTransform)) _rotationalpha true)))
        (:Finished
          (Variables|Default|SettileIndex (Utilities|Array|Get(acopy) (Variables|Default|GetPath%20Indexes)))
          (Utilities|Array|RemoveIndex (Variables|Default|GetPath%20Indexes))
          (if (> (Utilities|Array|Length (Variables|Default|GetPath%20Indexes)) 0)
            (goto _label)
            (else
              (Utilities|Array|RemoveIndex (Variables|Default|GetPath%20Between%20Grids))
              (if (> (Utilities|Array|Length (Variables|Default|GetPath%20Between%20Grids)) 0)
                (CallFunction|TeleportonTransition)
                (else
                  (CallFunction|SetAnimation "NewEnumerator0")))))))
      (else
        (Utilities|Array|RemoveIndex (Variables|Default|GetPath%20Between%20Grids))
        (if (> (Utilities|Array|Length (Variables|Default|GetPath%20Between%20Grids)) 0)
          (CallFunction|TeleportonTransition)
          (else
            (CallFunction|SetAnimation "NewEnumerator0")))))))

(event Custom|ResetPathIndexes_Event
  (bind _path_between_grids (Variables|Default|GetPath%20Between%20Grids))
  (bind _path_between_grids_2 (Variables|Default|GetPath%20Between%20Grids))
  (Variables|Default|SetPath%20Indexes (.index (Utilities|Array|Get(acopy) (Variables|Default|GetPath%20Between%20Grids))))
  (if (> (Utilities|Array|Length (Variables|Default|GetPath%20Indexes)) 0)
    (Variables|Default|SetcurrentTransform (Transformation|GetActorTransform) :!label _label)
    (Variables|Default|SettargetTransform (.transform (.Value (Utilities|Map|Find (Variables|/Game/BP/Core/Grid/BP_Grid.BP_Grid_C|GetgridTiles (Variables|Default|Getgrid)) (Utilities|Array|Get(acopy) (Variables|Default|GetPath%20Indexes))))))
    (Variables|Default|SettargetTransform (Math|Transform|MakeTransform (.location (Variables|Default|GettargetTransform)) (Math|Rotator|FindLookatRotation (.location (Variables|Default|GetcurrentTransform)) (.location (Variables|Default|GettargetTransform))) "1.000000,1.000000,1.000000"))
    (Components|Timeline|SetPlayRate (Variables|Default|GetmovementOnGrids) (Variables|Default|GetSpeed))
    (bind (_direction _time_alpha _rotationalpha) (Timeline|movementOnGrids PlayFromStart)
      (:Update
        (Transformation|SetActorLocation (Math|Vector|Lerp(Vector) (.location (Variables|Default|GetcurrentTransform)) (.location (Variables|Default|GettargetTransform)) _time_alpha) false false)
        (Transformation|SetActorRotation (Math|Rotator|Lerp(Rotator) (.rotation (Variables|Default|GetcurrentTransform)) (.rotation (Variables|Default|GettargetTransform)) _rotationalpha true)))
      (:Finished
        (Variables|Default|SettileIndex (Utilities|Array|Get(acopy) (Variables|Default|GetPath%20Indexes)))
        (Utilities|Array|RemoveIndex (Variables|Default|GetPath%20Indexes))
        (if (> (Utilities|Array|Length (Variables|Default|GetPath%20Indexes)) 0)
          (goto _label)
          (else
            (Utilities|Array|RemoveIndex _path_between_grids_2)
            (if (> (Utilities|Array|Length _path_between_grids_2) 0)
              (CallFunction|TeleportonTransition)
              (else
                (CallFunction|SetAnimation "NewEnumerator0")))))))
    (else
      (Utilities|Array|RemoveIndex _path_between_grids)
      (if (> (Utilities|Array|Length _path_between_grids) 0)
        (CallFunction|TeleportonTransition)
        (else
          (CallFunction|SetAnimation "NewEnumerator0"))))))

(event EventBeginPlay
  (CallFunction|TraceforGridandTileIndex)
  (Transformation|SetActorLocation (.location (.transform (Utilities|Struct|BreakS_TileData (.Value (Utilities|Map|Find (Variables|/Game/BP/Core/Grid/BP_Grid.BP_Grid_C|GetgridTiles (Variables|Default|Getgrid)) (Variables|Default|GettileIndex)))))) false false)
  (CallFunction|UpdateSelection))

(event Collision|EventActorBeginOverlap
  (params (OtherActor :type Actor%20Object%20Reference)))

(event EventTick
  (params (DeltaSeconds :type Float%20%28single-precision%29)))

(fn ConstructionScript
  (CallFunction|TraceforGridandTileIndex))

(fn UpdateMaterial
  (Rendering|Material|SetVectorParameterValueonMaterials (Variables|Default|GetCharMesh) "StateMultiply" (Utilities|Select :Index (Variables|Default|GetUIState) :NewEnumerator2 "1.000000,1.000000,1.000000" :NewEnumerator0 "1.000000,1.000000,1.000000" :NewEnumerator1 "6.000000,6.000000,6.000000")))

(fn UpdateSelection
  (Development|SetHiddeninGame (Variables|Default|GetSelectedArrow) (not (Variables|Default|Getselected)) false))

(fn TraceforGridandTileIndex
  (bind _returnvalue (Transformation|GetActorLocation))
  (bind _outhit (Collision|SphereTraceByChannel _returnvalue _returnvalue 5.0 "TraceTypeQuery4" false 0 "ForOneFrame"))
  (bind _asbp_grid_mesh_inst (Utilities|Casting|CastToBP_GridMeshInst (.HitActor (Collision|BreakHitResult _outhit))))
  (bind _outactors (Actor|GetAllActorsOfClass "/Game/BP/Core/Grid/BP_Grid.BP_Grid_C"))
  (bind _array_element (Utilities|Array|ForEachLoopwithBreak _outactors :!label _label)
    (:LoopBody
      (if (== (Variables|/Script/Engine.ChildActorComponent|GetChildActor (Variables|/Game/BP/Core/Utilities/BP_GridVisual.BP_GridVisual_C|GetCA_GridMeshInst (.AsBP%20Grid%20Visual (Utilities|Casting|CastToBP_GridVisual (Variables|/Script/Engine.ChildActorComponent|GetChildActor (Variables|/Game/BP/Core/Grid/BP_Grid.BP_Grid_C|GetCA_GridVisuals _array_element)))))) _asbp_grid_mesh_inst)
        (Variables|Default|Setgrid _array_element)
        (goto _label Break)))
    (:Completed
      (bind _index (Default|GetTileIndexfromWorldLoc (Variables|Default|Getgrid) (Transformation|GetActorLocation)))
      (bind _output_get (Variables|Default|SettileIndex _index))
      (return (Variables|Default|Getgrid) _output_get))))

(fn SetAnimation
  (params (anim :type E_CharAnimationStates%20Enum :default "NewEnumerator0"))
  (Class|BPIUnitAnimation|ChangeUnitAnimationState(Message) (Components|SkeletalMesh|GetAnimInstance (Variables|Default|GetCharMesh)) anim))

(fn TeleportonTransition
  (bind _outactors (Actor|GetAllActorsOfClass "/Game/BP/Core/Grid/BP_GridTransition.BP_GridTransition_C"))
  (bind _array_element (Utilities|Array|ForEachLoopwithBreak _outactors :!label _label)
    (:LoopBody
      (if (and (== (Variables|/Game/BP/Core/Grid/BP_GridModifier.BP_GridModifier_C|Getgrid _array_element) (Variables|Default|Getgrid)) (Class|KismetMathLibrary|EqualIntPointIntPoint (Utilities|Array|Get(acopy) (Variables|/Game/BP/Core/Grid/BP_GridModifier.BP_GridModifier_C|Getindexes _array_element)) (Variables|Default|GettileIndex)))
        (Variables|Default|Setgrid (Variables|/Game/BP/Core/Grid/BP_GridModifier.BP_GridModifier_C|Getgrid (Variables|/Game/BP/Core/Grid/BP_GridTransition.BP_GridTransition_C|GettoTile _array_element)))
        (Variables|Default|SettileIndex (Utilities|Array|Get(acopy) (Variables|/Game/BP/Core/Grid/BP_GridModifier.BP_GridModifier_C|Getindexes (Variables|/Game/BP/Core/Grid/BP_GridTransition.BP_GridTransition_C|GettoTile _array_element))))
        (Transformation|SetActorLocation (.location (.transform (.Value (Utilities|Map|Find (Variables|/Game/BP/Core/Grid/BP_Grid.BP_Grid_C|GetgridTiles (Variables|/Game/BP/Core/Grid/BP_GridModifier.BP_GridModifier_C|Getgrid (Variables|/Game/BP/Core/Grid/BP_GridTransition.BP_GridTransition_C|GettoTile _array_element))) (Utilities|Array|Get(acopy) (Variables|/Game/BP/Core/Grid/BP_GridModifier.BP_GridModifier_C|Getindexes (Variables|/Game/BP/Core/Grid/BP_GridTransition.BP_GridTransition_C|GettoTile _array_element))))))) false false)
        (goto _label Break)))
    (:Completed
      (CallFunction|ResetPathIndexesEvent))))