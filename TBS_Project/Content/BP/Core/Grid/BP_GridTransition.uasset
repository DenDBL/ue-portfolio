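; Grid transition actor with a static mesh that aligns itself to a 100-unit grid when constructed.
; The construction script snaps the mesh's world X and Y from the actor location, leaving Z unsnapped.
; BeginPlay only calls the parent, and an unconnected debug print references Grid and the first Indexes entry, so no transition logic lives in these graphs.
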(event EventBeginPlay
  (|CallParentFunction))

(event Collision|EventActorBeginOverlap
  (params (OtherActor :type Actor%20Object%20Reference))
  (|CallParentFunction OtherActor) ; This node is disabled and will not be called.\nDrag off pins to build functionality.
)

(event EventTick
  (params (DeltaSeconds :type Float%20%28single-precision%29))
  (|CallParentFunction DeltaSeconds) ; This node is disabled and will not be called.\nDrag off pins to build functionality.
)

(fn ConstructionScript
  (bind _returnvalue (Transformation|GetActorLocation))
  (bind _returnvector (CallFunction|SnapVectortoVector (Math|Vector|MakeVector (.x _returnvalue) (.y _returnvalue) (.z _returnvalue)) "100.000000,100.000000,100.000000"))
  (|CallParentFunction)
  (Transformation|SetWorldLocation (Variables|Default|GetStaticMesh) (Math|Vector|MakeVector (.x _returnvector) (.y _returnvector) (.z _returnvalue)) false false))