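; Pathfinder that finds a tile route between two positions that may lie on different grids linked by BP_GridTransition actors.
; A recursive search over all transitions collects chains from start grid to target grid.
; Each chain is expanded into per-grid segments through that grid's GridPathfinding, without diagonals.
; Candidates are compared by total index count to keep the shorter path, with a direct same-grid path as baseline when applicable.
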(event EventBeginPlay)

(event Collision|EventActorBeginOverlap
  (params (OtherActor :type Actor%20Object%20Reference)))

(event EventTick
  (params (DeltaSeconds :type Float%20%28single-precision%29)))

(fn ConstructionScript)

(fn FindPathBetweenGrids
  (params (startGrid :type BP%20Grid%20Object%20Reference) (targetGrid :type BP%20Grid%20Object%20Reference) (start :type Int%20Point%20Structure) (target :type Int%20Point%20Structure))
  (Variables|Default|SetstartIndex start)
  (Variables|Default|SettargetIndex target)
  (CallFunction|ClearPath)
  (if (== startGrid targetGrid)
    (CallFunction|GetPathonSameGrid startGrid)
    (LocalVariables|SetlengthOfPath (CallFunction|GetLengthOfPath (Variables|Default|GetcurrentPath))))
  (bind _returnpaths (CallFunction|FindTransitionPaths startGrid targetGrid))
  (if (Utilities|Array|IsEmpty _returnpaths)
    (return (Utilities|Array|MakeArray))
    (else
      (for _array_element _returnpaths
        (bind _returnpath (CallFunction|BuildPath _array_element))
        (if (< (CallFunction|GetLengthOfPath _returnpath) (LocalVariables|GetlengthOfPath))
          (bind _output_get (Variables|Default|SetcurrentPath _returnpath))
          (LocalVariables|SetlengthOfPath (CallFunction|GetLengthOfPath _output_get))))
      (return (Variables|Default|GetcurrentPath)))))

(fn GetAllTransitions
  (bind _outactors (Actor|GetAllActorsOfClass "/Game/BP/Core/Grid/BP_GridTransition.BP_GridTransition_C"))
  (return _outactors))

(fn FindTransitionPaths
  (params (startGrid :type BP%20Grid%20Object%20Reference) (targetGrid :type BP%20Grid%20Object%20Reference))
  (bind _array (Utilities|Array|MakeArray))
  (bind _transitionpaths (CallFunction|AnalyzeTransitions startGrid targetGrid _array _array))
  (return _transitionpaths))

(fn BuildPath
  (params (S_GridsPath :type S%20Grids%20Path%20Structure%20%28by%20ref%29))
  (bind _transitions (Utilities|Struct|BreakS_GridsPath S_GridsPath))
  (bind _output (Utilities|Array|Get(acopy) _transitions))
  (bind _grid (Variables|/Game/BP/Core/Grid/BP_GridModifier.BP_GridModifier_C|Getgrid _output))
  (bind _output_2 (Default|FindPath (Variables|/Game/BP/Core/Grid/BP_Grid.BP_Grid_C|GetGridPathfinding _grid) (Variables|Default|GetstartIndex) (Utilities|Array|Get(acopy) (Variables|/Game/BP/Core/Grid/BP_GridModifier.BP_GridModifier_C|Getindexes _output)) false))
  (Utilities|Array|Add (LocalVariables|Getpath) (Utilities|Struct|MakeS_IndexesAndGrid _output_2 _grid))
  (for (_array_element _array_index) _transitions
    (if (== _array_index (Utilities|Array|LastIndex _transitions))
      (bind _output_3 (Default|FindPath (Variables|/Game/BP/Core/Grid/BP_Grid.BP_Grid_C|GetGridPathfinding (Variables|/Game/BP/Core/Grid/BP_GridModifier.BP_GridModifier_C|Getgrid (Variables|/Game/BP/Core/Grid/BP_GridTransition.BP_GridTransition_C|GettoTile _array_element))) (Utilities|Array|Get(acopy) (Variables|/Game/BP/Core/Grid/BP_GridModifier.BP_GridModifier_C|Getindexes (Variables|/Game/BP/Core/Grid/BP_GridTransition.BP_GridTransition_C|GettoTile _array_element))) (Variables|Default|GettargetIndex) false))
      (Utilities|Array|Add (LocalVariables|Getpath) (Utilities|Struct|MakeS_IndexesAndGrid _output_3 (Variables|/Game/BP/Core/Grid/BP_GridModifier.BP_GridModifier_C|Getgrid (Variables|/Game/BP/Core/Grid/BP_GridTransition.BP_GridTransition_C|GettoTile _array_element))))
      (else
        (bind _output_4 (Default|FindPath (Variables|/Game/BP/Core/Grid/BP_Grid.BP_Grid_C|GetGridPathfinding (Variables|/Game/BP/Core/Grid/BP_GridModifier.BP_GridModifier_C|Getgrid (Utilities|Array|Get(acopy) _transitions (+ _array_index 1)))) (Utilities|Array|Get(acopy) (Variables|/Game/BP/Core/Grid/BP_GridModifier.BP_GridModifier_C|Getindexes (Variables|/Game/BP/Core/Grid/BP_GridTransition.BP_GridTransition_C|GettoTile _array_element))) (Utilities|Array|Get(acopy) (Variables|/Game/BP/Core/Grid/BP_GridModifier.BP_GridModifier_C|Getindexes (Utilities|Array|Get(acopy) _transitions (+ _array_index 1)))) false))
        (Utilities|Array|Add (LocalVariables|Getpath) (Utilities|Struct|MakeS_IndexesAndGrid _output_4 (Variables|/Game/BP/Core/Grid/BP_GridModifier.BP_GridModifier_C|Getgrid (Utilities|Array|Get(acopy) _transitions (+ _array_index 1))))))))
  (return (LocalVariables|Getpath)))

(fn GetLengthOfPath
  (params (path :type Array%20of%20S%20Indexes%20and%20Grid%20Structures))
  (for _array_element path
    (LocalVariables|Setlength (+ (Utilities|Array|Length (.index _array_element)) (LocalVariables|Getlength))))
  (return (LocalVariables|Getlength)))

(fn ClearPath
  (Utilities|Array|Clear (Variables|Default|GetcurrentPath))
  (Utilities|Array|Clear (Variables|Default|GettransitionPaths)))

(fn AnalyzeTransitions
  (params (beginGrid :type BP%20Grid%20Object%20Reference) (targetGrid :type BP%20Grid%20Object%20Reference) (path :type Array%20of%20BP%20Grid%20Transition%20Object%20References) (analyzedItems :type Array%20of%20BP%20Grid%20Transition%20Object%20References))
  (LocalVariables|SetlocalPath path)
  (LocalVariables|Setanalyzed analyzedItems)
  (for _array_element (CallFunction|GetAllTransitions)
    (LocalVariables|SetlocalPath path)
    (if (== (Variables|/Game/BP/Core/Grid/BP_GridModifier.BP_GridModifier_C|Getgrid _array_element) beginGrid)
      (if (not (Utilities|Array|ContainsItem (LocalVariables|Getanalyzed) _array_element))
        (Utilities|Array|Add (LocalVariables|GetlocalPath) _array_element)
        (Utilities|Array|Add (LocalVariables|Getanalyzed) _array_element)
        (LocalVariables|SetnextGrid (Variables|/Game/BP/Core/Grid/BP_GridModifier.BP_GridModifier_C|Getgrid (Variables|/Game/BP/Core/Grid/BP_GridTransition.BP_GridTransition_C|GettoTile _array_element)))
        (if (== (LocalVariables|GetnextGrid) targetGrid)
          (Utilities|Array|Add (Variables|Default|GettransitionPaths) (Utilities|Struct|MakeS_GridsPath 0 (LocalVariables|GetlocalPath))))
        (CallFunction|AnalyzeTransitions (LocalVariables|GetnextGrid) targetGrid (LocalVariables|GetlocalPath) (LocalVariables|Getanalyzed))
        (Utilities|Array|Clear (LocalVariables|GetlocalPath)))))
  (return (Variables|Default|GettransitionPaths)))

(fn GetGridsTransitions
  (params (grid :type BP%20Grid%20Object%20Reference) (t :type Array%20of%20BP%20Grid%20Transition%20Object%20References))
  (for _array_element t
    (if (== (Variables|/Game/BP/Core/Grid/BP_GridModifier.BP_GridModifier_C|Getgrid _array_element) grid)
      (Utilities|Array|Add (LocalVariables|Getreturn) _array_element)))
  (return (LocalVariables|Getreturn)))

(fn GetPathonSameGrid
  (params (grid :type BP%20Grid%20Object%20Reference))
  (bind _output (Default|FindPath (Variables|/Game/BP/Core/Grid/BP_Grid.BP_Grid_C|GetGridPathfinding grid) (Variables|Default|GetstartIndex) (Variables|Default|GettargetIndex) false))
  (Variables|Default|SetcurrentPath (Utilities|Array|MakeArray (Utilities|Struct|MakeS_IndexesAndGrid _output grid))))