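; Grid pathfinding Blueprint that runs an A*-style search between two tiles, with optional diagonal movement.
; FindPath validates both ends, then expands tiles from an open list kept sorted by cost plus Manhattan or Chebyshev estimate.
; It stops when the target is discovered and walks previous-index links back to return the path, excluding the start.
; Neighbor filtering checks walkability of the expanded tile, not of each neighbor.
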(event EventBeginPlay)

(event Collision|EventActorBeginOverlap
  (params (OtherActor :type Actor%20Object%20Reference)))

(event EventTick
  (params (DeltaSeconds :type Float%20%28single-precision%29)))

(fn ConstructionScript)

(fn GetNeighborTilesIndexes
  (params (Index :type Int%20Point%20Structure) (includeDiagonals :type Boolean))
  (Utilities|Array|AppendArray (LocalVariables|GetreturnIndexes) (Utilities|Array|MakeArray (+ Index (Utilities|Struct|MakeIntPoint 1 0)) (+ Index (Utilities|Struct|MakeIntPoint -1 0)) (+ Index (Utilities|Struct|MakeIntPoint 0 1)) (+ Index (Utilities|Struct|MakeIntPoint 0 -1))))
  (Utilities|FlowControl|Sequence
    (:then_0
      (if includeDiagonals
        (Utilities|Array|AppendArray (LocalVariables|GetreturnIndexes) (Utilities|Array|MakeArray (+ Index (Utilities|Struct|MakeIntPoint 1 1)) (+ Index (Utilities|Struct|MakeIntPoint -1 1)) (+ Index (Utilities|Struct|MakeIntPoint 1 -1)) (+ Index (Utilities|Struct|MakeIntPoint -1 -1))))))
    (:then_1
      (return (LocalVariables|GetreturnIndexes)))))

(fn GetValidNeighborTilesIndexes
  (params (index :type Int%20Point%20Structure) (includeDiagonals :type Boolean))
  (bind _indexes (CallFunction|GetNeighborTilesIndexes index includeDiagonals))
  (for _array_element _indexes
    (if (Default|IsWalkable (Variables|Default|Getgrid) (.type (.Value (Utilities|Map|Find (Variables|/Game/BP/Core/Grid/BP_Grid.BP_Grid_C|GetgridTiles (Variables|Default|Getgrid)) index))))
      (Utilities|Array|Add (LocalVariables|GetreturnIndexes) (Utilities|Struct|MakeS_PathFindingData _array_element 0 0 0 "(X=0,Y=0)"))))
  (return (LocalVariables|GetreturnIndexes)))

(fn FindPath
  (params (start :type Int%20Point%20Structure) (target :type Int%20Point%20Structure) (includeDiagonals :type Boolean))
  (Variables|Default|SetstartIndex start)
  (Variables|Default|SettargetIndex target)
  (Variables|Default|SetInclude%20Diagonals includeDiagonals)
  (CallFunction|ClearGeneratedData)
  (bind _valid (CallFunction|IsInputDataValid))
  (if _valid
    (CallFunction|DiscoverTile (Utilities|Struct|MakeS_PathFindingData (Variables|Default|GetstartIndex) 1 0 (CallFunction|GetMinimumCostBetweenTwoTiles (Variables|Default|GetstartIndex) (Variables|Default|GettargetIndex) (Variables|Default|GetInclude%20Diagonals)) "(X=0,Y=0)"))
    (while (> (Utilities|Array|Length (Variables|Default|GetdiscoveredTiles)) 0)
      (bind _foundtargettile (CallFunction|AnalyzeNextDiscoveredTile))
      (if _foundtargettile
        (bind _path (CallFunction|GeneratePath))
        (return _path)))
    (return (Utilities|Array|MakeArray))
    (else
      (return (Utilities|Array|MakeArray)))))

(fn IsInputDataValid
  (bind _grid (Variables|Default|Getgrid))
  (bind _grid_2 (Variables|Default|Getgrid))
  (if (!= (Variables|Default|GetstartIndex) (Variables|Default|GettargetIndex))
    (if (Default|IsWalkable _grid_2 (.type (.Value (Utilities|Map|Find (Variables|/Game/BP/Core/Grid/BP_Grid.BP_Grid_C|GetgridTiles _grid_2) (Variables|Default|GettargetIndex)))))
      (if (Default|IsWalkable _grid (.type (.Value (Utilities|Map|Find (Variables|/Game/BP/Core/Grid/BP_Grid.BP_Grid_C|GetgridTiles _grid) (Variables|Default|GetstartIndex)))))
        (return true)
        (else
          (return false)))
      (else
        (return false)))
    (else
      (return false))))

(fn DiscoverTile
  (params (Tile%20Path%20Data :type S%20Path%20Finding%20Data%20Structure))
  (Utilities|Map|Add (Variables|Default|GetpathfindingData) (.index (Utilities|Struct|BreakS_PathFindingData Tile%20Path%20Data)) Tile%20Path%20Data)
  (CallFunction|InsertTileinDiscoveredArr Tile%20Path%20Data))

(fn GetMinimumCostBetweenTwoTiles
  (params (index%201 :type Int%20Point%20Structure) (index%202 :type Int%20Point%20Structure) (diagonals :type Boolean))
  (bind _returnvalue (- index%201 index%202))
  (bind _returnvalue_2 (- index%201 index%202))
  (if diagonals
    (return (Math|Integer|Max(Integer) (Math|Integer|Absolute(Integer) (.x _returnvalue_2)) (Math|Integer|Absolute(Integer) (.y _returnvalue_2))))
    (else
      (return (+ (Math|Integer|Absolute(Integer) (.x _returnvalue)) (Math|Integer|Absolute(Integer) (.y _returnvalue)))))))

(fn AnalyzeNextDiscoveredTile
  (bind _tile_path_data (CallFunction|CheapestTilefromDiscovered))
  (Variables|Default|SetcurrentDiscoveredTile _tile_path_data)
  (bind _indexes (CallFunction|GetValidNeighborTilesIndexes (.index (Utilities|Struct|BreakS_PathFindingData (Variables|Default|GetcurrentDiscoveredTile))) (Variables|Default|GetInclude%20Diagonals)))
  (bind _output_get (Variables|Default|SetcurrentNeighbors _indexes))
  (while (> (Utilities|Array|Length _output_get) 0)
    (bind _istargertile (CallFunction|DiscoverNextNeighbor))
    (if _istargertile
      (return true)))
  (return false))

(fn GeneratePath
  (LocalVariables|Setcurent (Variables|Default|GettargetIndex))
  (while (!= (LocalVariables|Getcurent) (Variables|Default|GetstartIndex))
    (Utilities|Array|Add (LocalVariables|GetinvertedPath) (LocalVariables|Getcurent))
    (LocalVariables|Setcurent (.previuousindex (.Value (Utilities|Map|Find (Variables|Default|GetpathfindingData) (LocalVariables|Getcurent))))))
  (bind _arrayelement (Utilities|Array|ReverseforEachLoop (LocalVariables|GetinvertedPath))
    (:LoopBody
      (Utilities|Array|Add (LocalVariables|Getreturn) _arrayelement))
    (:Completed
      (return (LocalVariables|Getreturn)))))

(fn CheapestTilefromDiscovered
  (LocalVariables|SettileIndex (Utilities|Array|Get(acopy) (Variables|Default|GetdiscoveredTiles)))
  (Utilities|Array|RemoveIndex (Variables|Default|GetdiscoveredTilesSortingCosts))
  (Utilities|Array|RemoveIndex (Variables|Default|GetdiscoveredTiles))
  (Utilities|Array|Add (Variables|Default|GetanalyzedTiles) (LocalVariables|GettileIndex))
  (return (.Value (Utilities|Map|Find (Variables|Default|GetpathfindingData) (LocalVariables|GettileIndex)))))

(fn DiscoverNextNeighbor
  (Variables|Default|SetcurrentNeighbor (Utilities|Array|Get(acopy) (Variables|Default|GetcurrentNeighbors)))
  (Utilities|Array|RemoveIndex (Variables|Default|GetcurrentNeighbors))
  ;[1 1 1] Еще не анализирована?
  (if (not (Utilities|Array|ContainsItem (Variables|Default|GetanalyzedTiles) (.index (Variables|Default|GetcurrentNeighbor))))
    (LocalVariables|SetcostFromStart (+ (.costFromStart (Utilities|Struct|BreakS_PathFindingData (Variables|Default|GetcurrentDiscoveredTile))) (.costToEnterTile (Utilities|Struct|BreakS_PathFindingData (Variables|Default|GetcurrentNeighbor)))))
    (bind _output_get (LocalVariables|SetindexInDiscovered (Utilities|Array|FindItem (Variables|Default|GetdiscoveredTiles) (.index (Variables|Default|GetcurrentNeighbor)))))
    (if (== _output_get -1) ; Новая соседняя клетка?
      _
      (else
        (bind _output_get_2 (Variables|Default|SetcurrentNeighbor (.Value (Utilities|Map|Find (Variables|Default|GetpathfindingData) (.index (Utilities|Struct|BreakS_PathFindingData (Variables|Default|GetcurrentNeighbor)))))))
        (if (< (LocalVariables|GetcostFromStart) (.costFromStart (Utilities|Struct|BreakS_PathFindingData _output_get_2)))
          (Utilities|Array|RemoveIndex (Variables|Default|GetdiscoveredTiles) (LocalVariables|GetindexInDiscovered))
          (Utilities|Array|RemoveIndex (Variables|Default|GetdiscoveredTilesSortingCosts) (LocalVariables|GetindexInDiscovered))
          (else
            (return false)))))
    (CallFunction|DiscoverTile (Utilities|Struct|MakeS_PathFindingData (.index (Utilities|Struct|BreakS_PathFindingData (Variables|Default|GetcurrentNeighbor))) (.costToEnterTile (Utilities|Struct|BreakS_PathFindingData (Variables|Default|GetcurrentNeighbor))) (LocalVariables|GetcostFromStart) (CallFunction|GetMinimumCostBetweenTwoTiles (.index (Utilities|Struct|BreakS_PathFindingData (Variables|Default|GetcurrentNeighbor))) (Variables|Default|GettargetIndex) (Variables|Default|GetInclude%20Diagonals)) (.index (Variables|Default|GetcurrentDiscoveredTile))))
    (if (Class|KismetMathLibrary|EqualIntPointIntPoint (.index (Utilities|Struct|BreakS_PathFindingData (Variables|Default|GetcurrentNeighbor))) (Variables|Default|GettargetIndex))
      (return true)
      (else
        (return false)))
    (else
      (return false))))

(fn InsertTileinDiscoveredArr
  (params (tileData :type S%20Path%20Finding%20Data%20Structure))
  (bind (_index _costtoentertile _costfromstart _minimumcostfromstart) (Utilities|Struct|BreakS_PathFindingData tileData))
  (bind _discoveredtilessortingcosts (Variables|Default|GetdiscoveredTilesSortingCosts))
  (LocalVariables|SetsortCost (+ _costfromstart _minimumcostfromstart))
  (if (== (Utilities|Array|Length (Variables|Default|GetdiscoveredTilesSortingCosts)) 0)
    (Utilities|Array|Add (Variables|Default|GetdiscoveredTilesSortingCosts) (LocalVariables|GetsortCost) :!label _label)
    (Utilities|Array|Add (Variables|Default|GetdiscoveredTiles) (.index tileData))
    (elif (>= (LocalVariables|GetsortCost) (Utilities|Array|Get(acopy) _discoveredtilessortingcosts (Utilities|Array|LastIndex _discoveredtilessortingcosts)))
      (goto _label)
      (else
        (bind (_array_element _array_index) (Utilities|Array|ForEachLoopwithBreak (Variables|Default|GetdiscoveredTilesSortingCosts) :!label _label_2)
          (:LoopBody
            (if (>= _array_element (LocalVariables|GetsortCost))
              (Utilities|Array|Insert (Variables|Default|GetdiscoveredTilesSortingCosts) (LocalVariables|GetsortCost) _array_index)
              (Utilities|Array|Insert (Variables|Default|GetdiscoveredTiles) (.index tileData) _array_index)
              (goto _label_2 Break))))))))

(fn ClearGeneratedData
  (Utilities|FlowControl|Sequence
    (:then_0
      (Utilities|Map|Clear (Variables|Default|GetpathfindingData)))
    (:then_1
      (Utilities|Array|Clear (Variables|Default|GetdiscoveredTilesSortingCosts)))
    (:then_2
      (Utilities|Array|Clear (Variables|Default|GetdiscoveredTiles)))
    (:then_3
      (Utilities|Array|Clear (Variables|Default|GetanalyzedTiles)))))