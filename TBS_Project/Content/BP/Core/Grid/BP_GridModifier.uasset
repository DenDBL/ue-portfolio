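; Grid modifier actor that represents a tile type, such as obstacle or transition, as a colored square mesh.
; Its construction script pulls the Square mesh from DT_GridShapeDatatable, tints it by TileType and applies the HiddenInGame setting.
; The mesh overlaps a custom trace channel, ignores pawns and cannot be stepped on.
; Event graph logic is empty; a helper function clears the stored Indexes.
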(event EventBeginPlay)

(event Collision|EventActorBeginOverlap
  (params (OtherActor :type Actor%20Object%20Reference)))

(event EventTick
  (params (DeltaSeconds :type Float%20%28single-precision%29)))

(fn ConstructionScript
  (bind _returnvalue (Utilities|GetDataTableRow "/Game/BP/Core/Grid/GridShapes/DT_GridShapeDatatable.DT_GridShapeDatatable" "Square")
    (:then
      (Components|StaticMesh|SetStaticMesh (Variables|Default|GetStaticMesh) (.mesh _returnvalue))
      (Rendering|Material|SetVectorParameterValueonMaterials (Variables|Default|GetStaticMesh) "Color" (Math|Conversions|ToVector(LinearColor) (Utilities|Select :Index (Variables|Default|GettileType) :NewEnumerator0 "" :NewEnumerator1 "(R=1.000000,G=1.000000,B=1.000000,A=1.000000)" :NewEnumerator2 "(R=1.000000,G=0.000000,B=0.034921,A=1.000000)" :NewEnumerator3 "(R=1.000000,G=0.000000,B=0.924858,A=1.000000)")))
      (Collision|SetCollisionResponsetoChannel (Variables|Default|GetStaticMesh) "ECC_GameTraceChannel1" "ECR_Overlap")
      (Rendering|SetActorHiddenInGame (Variables|Default|GethiddenInGame))
      (Collision|SetCollisionResponsetoChannel (Variables|Default|GetStaticMesh) "ECC_Pawn" "ECR_Ignore")
      (Variables|/Script/Engine.PrimitiveComponent|SetCanCharacterStepUpOn (Variables|Default|GetStaticMesh) "ECB_No"))))

(fn ClearIndexes
  (Utilities|Array|Clear (Variables|Default|Getindexes)))