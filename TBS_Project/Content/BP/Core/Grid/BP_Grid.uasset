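; BP_Grid is the core square tile grid actor, storing each tile's type, transform and states by index.
; Its construction script builds the centered grid and connects child visual and pathfinding actors.
; Optional sphere traces type tiles from ground and overlapping BP_GridModifiers, which record covered indices; BeginPlay always retraces.
; Helpers map cursor hits, with plane-intersection fallback, to indices and edit tile states, updating visuals and signaling changes.
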(event EventBeginPlay
  (bind _keys (Utilities|Map|Keys (Variables|Default|GetgridTiles)))
  (for _array_element _keys
    (Default|CallOnTileDataUpdate _array_element self))
  (bind _keys_2 (Utilities|Map|Keys (Variables|Default|GetgridTiles)))
  (for _array_element_2 _keys_2
    (bind _tiletype (CallFunction|TraceforGround (.Location (Math|Transform|BreakTransform (.transform (Utilities|Struct|BreakS_TileData (.Value (Utilities|Map|Find (Variables|Default|GetgridTiles) _array_element_2)))))) (.index (Utilities|Struct|BreakS_TileData (.Value (Utilities|Map|Find (Variables|Default|GetgridTiles) _array_element_2))))))
    (Utilities|Map|Add (Variables|Default|GetgridTiles) _array_element_2 (Utilities|Struct|MakeS_TileData _array_element_2 _tiletype (.transform (Utilities|Struct|BreakS_TileData (.Value (Utilities|Map|Find (Variables|Default|GetgridTiles) _array_element_2)))) (.tileState (Utilities|Struct|BreakS_TileData (.Value (Utilities|Map|Find (Variables|Default|GetgridTiles) _array_element_2))))))))

(event Collision|EventActorBeginOverlap
  (params (OtherActor :type Actor%20Object%20Reference)))

(event EventTick
  (params (DeltaSeconds :type Float%20%28single-precision%29)))

(fn ConstructionScript
  (Variables|Default|SetgridVisual (.AsBP%20Grid%20Visual (Utilities|Casting|CastToBP_GridVisual (Variables|/Script/Engine.ChildActorComponent|GetChildActor (Variables|Default|GetCA_GridVisuals)))))
  (bind _output_get (Variables|Default|SetGridPathfinding (.AsBP%20Grid%20Pathfinding (Utilities|Casting|CastToBP_GridPathfinding (Variables|/Script/Engine.ChildActorComponent|GetChildActor (Variables|Default|GetCA_Pathfinding))))))
  (Variables|/Game/BP/Core/Grid/BP_GridPathfinding.BP_GridPathfinding_C|Setgrid _output_get self)
  (CallFunction|SpawnGrid (Transformation|GetActorLocation) (Variables|Default|GetgridTileSize) (Variables|Default|GetgridTileCount)))

(fn SpawnGrid
  (params (centerLocation :type Vector) (tileSize :type Vector) (tileCount :type Int%20Point%20Structure))
  (bind _center (CallFunction|FindCenterandBottomLeftCornerLoc))
  ;[1 1 1] Передаем параметры сетки
  (Variables|Default|SetgridCenterLocation centerLocation)
  (Variables|Default|SetgridTileSize tileSize)
  (Variables|Default|SetgridTileCount tileCount)
  (CallFunction|DestroyGrid)
  ;[1 1 1] Задаём меш
  (Default|InitGridVisuals (Variables|Default|GetgridVisual))
  ;[1 1 1] Находим центр сетки
  (Variables|Default|SetgridCenterLocation (Math|Vector|MakeVector (.x _center) (.y _center) (.z centerLocation)))
  ;[1 1 1] Находим позицию нижнего левого угла сетки
  (Variables|Default|SetgridBottomLeftCornerLocation (.BottomLeftCornerLoc (CallFunction|FindCenterandBottomLeftCornerLoc)))
  ;[1 1 1] Цикл по X
  (for _index (range 0 (Math|Float|Truncate (Math|Conversions|ToFloat(Integer) (- (.x (Variables|Default|GetgridTileCount)) 1))))
    (LocalVariables|Setx _index)
    ;[1 1 1] Цикл по Y
    (for _index_2 (range 0 (Math|Float|Truncate (Math|Conversions|ToFloat(Integer) (- (.y (Variables|Default|GetgridTileCount)) 1))))
      (LocalVariables|Sety _index_2)
      (bind _returnvalue (Utilities|GetDataTableRow "/Game/BP/Core/Grid/GridShapes/DT_GridShapeDatatable.DT_GridShapeDatatable" "Square")
        (:then
          ;[1 1 1] Задаём позицию и размер тайла
          (LocalVariables|SettileTransform (Math|Transform|MakeTransform (+ (Variables|Default|GetgridBottomLeftCornerLocation) (* (Variables|Default|GetgridTileSize) (Math|Vector|MakeVector (Math|Conversions|ToFloat(Integer) (LocalVariables|Getx)) (Math|Conversions|ToFloat(Integer) (LocalVariables|Gety)) 0.0))) "0, 0, 0" (/ (Variables|Default|GetgridTileSize) (.meshsize _returnvalue))))
          (if (Variables|Default|GetgroundTrace)
            ;[1 1 1] Поверхность под клетками и наличие препятствия
            (bind _tiletype (CallFunction|TraceforGround (.location (LocalVariables|GettileTransform)) (Utilities|Struct|MakeIntPoint (LocalVariables|Getx) (LocalVariables|Gety))))
            (CallFunction|AddGridTile (Utilities|Struct|MakeS_TileData (Utilities|Struct|MakeIntPoint (LocalVariables|Getx) (LocalVariables|Gety)) _tiletype (LocalVariables|GettileTransform) "(INVALID)"))
            (else
              ;[1 1 1] Добавляем тайл
              (CallFunction|AddGridTile (Utilities|Struct|MakeS_TileData (Utilities|Struct|MakeIntPoint (LocalVariables|Getx) (LocalVariables|Gety)) "NewEnumerator1" (LocalVariables|GettileTransform) "(INVALID)")))))))))

(fn FindCenterandBottomLeftCornerLoc
  (bind _gridtilecount (Variables|Default|GetgridTileCount))
  (return (- (Variables|Default|GetgridCenterLocation) (* (/ (- (Variables|Default|GetgridTileCount) (Math|Vector2D|MakeVector2D (Math|Float|SelectFloat 0.0 1.0 (CallFunction|IsEven(Float) (Math|Conversions|ToFloat(Integer) (.x _gridtilecount)))) (Math|Float|SelectFloat 0.0 1.0 (CallFunction|IsEven(Float) (Math|Conversions|ToFloat(Integer) (.y _gridtilecount)))))) "(X=2.000000,Y=2.000000)") (Variables|Default|GetgridTileSize))) (CallFunction|SnapVectortoVector (Variables|Default|GetgridCenterLocation) (Variables|Default|GetgridTileSize))))

(fn TraceforGround
  (params (tileLoc :type Vector) (index :type Int%20Point%20Structure))
  (LocalVariables|Settype "NewEnumerator0")
  (bind (_outhits _returnvalue) (Collision|MultiSphereTraceByChannel (+ tileLoc (Math|Vector|MakeVector 0.0 0.0 -1e+01)) (+ tileLoc (Math|Vector|MakeVector 0.0 0.0 1e+01)) (/ (.x (Variables|Default|GetgridTileSize)) 3.0) "TraceTypeQuery3" false 0 "ForOneFrame"))
  (if _returnvalue
    (LocalVariables|Settype "NewEnumerator1")
    (for _array_element _outhits
      (Utilities|FlowControl|Sequence
        (:then_0
          (bind _asbp_grid_modifier (Utilities|Casting|CastToBP_GridModifier (.HitActor (Collision|BreakHitResult _array_element))))
          (LocalVariables|Settype (Variables|/Game/BP/Core/Grid/BP_GridModifier.BP_GridModifier_C|GettileType _asbp_grid_modifier))
          (Variables|/Game/BP/Core/Grid/BP_GridModifier.BP_GridModifier_C|Setgrid _asbp_grid_modifier self)
          (Utilities|Array|AddUnique (Variables|/Game/BP/Core/Grid/BP_GridModifier.BP_GridModifier_C|Getindexes _asbp_grid_modifier) index))))
    (return "0, 0, 0" (LocalVariables|Gettype))
    (else
      (return "0, 0, 0" (LocalVariables|Gettype)))))

(fn IsWalkable
  (params (type :type E_TypeOfTile%20Enum :default "NewEnumerator0"))
  (return (not (Utilities|Array|ContainsItem (Utilities|Array|MakeArray "NewEnumerator0" "NewEnumerator2") type))))

(fn AddGridTile
  (params (data :type S%20Tile%20Data%20Structure%20%28by%20ref%29))
  (Utilities|Map|Add (Variables|Default|GetgridTiles) (.index data) data)
  (Default|UpdateTileVisual (Variables|Default|GetgridVisual) data)
  (Default|CallOnTileDataUpdate (.index data) self))

(fn DestroyGrid
  (Utilities|Map|Clear (Variables|Default|GetgridTiles))
  (Default|DestroyGridVisual (Variables|Default|GetgridVisual)))

(fn GetCursorLocationonGrid
  (params (PlayerIndex :type Integer))
  (bind _returnvalue (Game|GetPlayerController PlayerIndex))
  (bind _gridcenterlocation (Variables|Default|GetgridCenterLocation))
  (bind (_hitresult _returnvalue_2) (Game|Player|GetHitResultUnderCursorbyChannel _returnvalue "TraceTypeQuery4" false))
  (bind (_worldlocation _worlddirection) (Game|Player|ConvertMouseLocationToWorldSpace _returnvalue))
  (bind _returnvalue_3 (Class|KismetMathLibrary|MakePlanefromPointandNormal _gridcenterlocation "0, 0,1.000000"))
  (bind _returnvalue_4 (* _worlddirection 99999.0))
  (bind _returnvalue_5 (+ _worldlocation _returnvalue_4))
  (bind (_t _intersection _returnvalue_6) (Class|KismetMathLibrary|LinePlaneIntersection _worldlocation _returnvalue_5 _returnvalue_3))
  (if _returnvalue_2
    (return (.Location (Collision|BreakHitResult _hitresult)))
    (elif _returnvalue_6
      (return _intersection)
      (else
        (return "-999.000000,-999.000000,-999.000000")))))

(fn GetTileIndexfromWorldLoc
  (params (Location :type Vector))
  (bind _gridtilesize (Variables|Default|GetgridTileSize))
  (LocalVariables|SetlocationOnGrid (- Location (Variables|Default|GetgridBottomLeftCornerLocation)))
  (bind _output_get (Variables|Default|SetsnappedLocOnGrid (Math|Conversions|ToVector2D(Vector) (CallFunction|SnapVectortoVector (LocalVariables|GetlocationOnGrid) (Variables|Default|GetgridTileSize)))))
  (return (Class|KismetMathLibrary|ToIntPoint(Vector2D) (/ _output_get (Math|Vector2D|MakeVector2D (.x _gridtilesize) (.y _gridtilesize))))))

(fn GetTileIndexUnderCursor
  (params (PlayerIndex :type Integer))
  (bind _index (CallFunction|GetTileIndexfromWorldLoc (CallFunction|GetCursorLocationonGrid PlayerIndex)))
  (return _index))

(fn AddGridTileState
  (params (index :type Int%20Point%20Structure) (state :type E_TileState%20Enum :default "NewEnumerator0"))
  (bind _gridtiles (Variables|Default|GetgridTiles))
  (bind (_value _returnvalue) (Utilities|Map|Find _gridtiles index))
  ;[1 1 1] Находим тайл в списке
  (if _returnvalue
    ;[1 1 1] Локальная переменная с параметрами тайла. Задаем в неё переданное состояние
    (bind _output_get (LocalVariables|Setdata _value))
    (bind _returnvalue_2 (Utilities|Array|AddUnique (.tilestate _output_get) state))
    ;[1 1 1] Если что-то было переданно
    (if (>= _returnvalue_2 0)
      ;[1 1 1] Обновляем данные тайла
      (Utilities|Map|Add (Variables|Default|GetgridTiles) (.index (LocalVariables|Getdata)) (LocalVariables|Getdata))
      ;[1 1 1] Обновялем визуал тайла
      (Default|UpdateTileVisual (Variables|Default|GetgridVisual) (LocalVariables|Getdata))
      (Default|CallOnTileDataUpdate (.index (LocalVariables|Getdata)) self))))

(fn RemoveGridTileState
  (params (index :type Int%20Point%20Structure) (state :type E_TileState%20Enum :default "NewEnumerator0"))
  (bind _gridtiles (Variables|Default|GetgridTiles))
  (bind (_value _returnvalue) (Utilities|Map|Find _gridtiles index))
  ;[1 1 1] Находим тайл в списке
  (if _returnvalue
    ;[1 1 1] Локальная переменная с параметрами тайла. Удаляем переданное состояние
    (bind _output_get (LocalVariables|Setdata _value))
    (bind _returnvalue_2 (Utilities|Array|RemoveItem (.tilestate _output_get) state))
    ;[1 1 1] Если что-то было удалено
    (if _returnvalue_2
      ;[1 1 1] Обновляем данные тайла
      (Utilities|Map|Add (Variables|Default|GetgridTiles) (.index (LocalVariables|Getdata)) (LocalVariables|Getdata))
      ;[1 1 1] Обновялем визуал тайла
      (Default|UpdateTileVisual (Variables|Default|GetgridVisual) (LocalVariables|Getdata))
      (Default|CallOnTileDataUpdate (.index (LocalVariables|Getdata)) self))))

(fn GetTileswithState
  (params (state :type E_TileState%20Enum :default "NewEnumerator0"))
  (bind _values (Utilities|Map|Values (Variables|Default|GetgridTiles)))
  (for _array_element _values
    (if (Utilities|Array|ContainsItem (.tilestate _array_element) state)
      (Utilities|Array|Add (LocalVariables|GetInd) (.index _array_element))))
  (return (LocalVariables|GetInd)))

(fn ClearStatefromTiles
  (params (state :type E_TileState%20Enum :default "NewEnumerator0"))
  (bind _indexes (CallFunction|GetTileswithState state))
  (for _array_element _indexes
    (CallFunction|RemoveGridTileState _array_element state)))