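; BP_PlayerActions is the player's mouse input actor for selecting and moving units across multiple BP_Grid grids.
; Tick traces for the unit under the cursor and, with a unit selected, highlights the hovered tile, switching grids and playing a snap sound.
; Clicks delegate to spawned, swappable action actors: left runs unit selection and clears tile states, right runs tile-select and move-between-grids on walkable tiles.
; A child actor supplies the cross-grid pathfinding reference.
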(event EventBeginPlay
  (Input|EnableInput (Game|GetPlayerController 0))
  ;[1 1 1] массив сеток
  (bind _outactors (Actor|GetAllActorsOfClass "/Game/BP/Core/Grid/BP_Grid.BP_Grid_C"))
  (bind _output_get (Variables|Default|SetGrids _outactors))
  (if (> (Utilities|Array|Length _output_get) 0)
    ;[1 1 1] Начальное значение выбранной сетки
    (Variables|Default|SethoveredGrid (Utilities|Array|Get(acopy) _output_get))
    (Variables|Default|SetselectedGrid (Utilities|Array|Get(acopy) _output_get)))
  ;[1 1 1] Задаём действия для кнопок мыши
  (CallFunction|SetSelectedActions "/Game/BP/Core/Player/Actions/Action_SelectTile.Action_SelectTile_C" "/Game/BP/Core/Player/Actions/Action_SelectTile.Action_SelectTile_C")
  (bind _returnvalue (Game|SpawnActorfromClass "/Game/BP/Core/Player/UnitActions/UnitAction_SelectUnit.UnitAction_SelectUnit_C" (Math|Transform|MakeTransform "0, 0, 0" "0, 0, 0" "1.000000,1.000000,1.000000") "Undefined" 0 self 0))
  (Variables|Default|SetUnitAction_LMB _returnvalue)
  (bind _returnvalue_2 (Game|SpawnActorfromClass "/Game/BP/Core/Player/UnitActions/UnitAction_MoveUnitBetweenGrids.UnitAction_MoveUnitBetweenGrids_C" (Math|Transform|MakeTransform "0, 0, 0" "0, 0, 0" "1.000000,1.000000,1.000000") "Undefined" 0 self 0))
  (Variables|Default|SetUnitAction_RMB _returnvalue_2))

(event EventTick
  (params (DeltaSeconds :type Float%20%28single-precision%29))
  (Utilities|FlowControl|Sequence
    (:then_0
      (CallFunction|UpdateUnitUndertheCursor))
    (:then_1
      (Utilities|IsValid (Variables|Default|GetselectedUnit)
        (:Is%20Valid
          (CallFunction|UpdateTileUndertheCursor))))))

(event Input|MouseEvents|LeftMouseButton
  (params (Key :type Key%20Structure :default "None"))
  (:Pressed
    (Utilities|FlowControl|Sequence
      (:then_0
        (CallFunction|UpdateUnitUndertheCursor)
        (Default|Exec (Variables|Default|GetUnitAction_LMB) (Variables|Default|GethoveredUnit))
        (CallFunction|ResetHoveredTile)
        (for _array_element (Variables|Default|GetGrids)
          (Default|ClearStatefromTiles _array_element "NewEnumerator4")
          (Default|ClearStatefromTiles _array_element "NewEnumerator2"))))))

(event Input|MouseEvents|RightMouseButton
  (params (Key :type Key%20Structure :default "None"))
  (:Pressed
    (Utilities|IsValid (Variables|Default|GetSelectedAction_RMB)
      (:Is%20Valid
        (Utilities|IsValid (Variables|Default|GetselectedUnit)
          (:Is%20Valid
            (CallFunction|UpdateTileUndertheCursor)
            (if (CallFunction|IsTileTypeWalkable (.type (.Value (Utilities|Map|Find (Variables|/Game/BP/Core/Grid/BP_Grid.BP_Grid_C|GetgridTiles (Variables|Default|GethoveredGrid)) (Variables|Default|GethoveredTileOfHoveredGrid)))))
              (Default|ExecAction (Variables|Default|GetSelectedAction_RMB) (Variables|Default|GethoveredTileOfHoveredGrid))
              (Default|Exec (Variables|Default|GetUnitAction_RMB) (Variables|Default|GetselectedUnit)))))))))

(fn ConstructionScript
  (Variables|Default|SetgridsPathfinding (.AsBP%20Grids%20Pathfinding (Utilities|Casting|CastToBP_GridsPathfinding (Variables|/Script/Engine.ChildActorComponent|GetChildActor (Variables|Default|GetCA_PathfindingBetweenGrids))))))

(fn UpdateTileUndertheCursor
  (if (Utilities|IsValid (Variables|Default|GethoveredGrid))
    ;[1 1 1] Получаем тайл активной сетки
    (bind _index (Default|GetTileIndexUnderCursor (Variables|Default|GethoveredGrid)))
    ;[1 1 1] Если это не тот же самый тайл
    (if (!= _index (Variables|Default|GethoveredTileOfHoveredGrid))
      ;[1 1 1] Убираем статус клетк
      (Default|RemoveGridTileState (Variables|Default|GethoveredGrid) (Variables|Default|GethoveredTileOfHoveredGrid) "NewEnumerator1")
      ;[1 1 1] Задаем новую активную сетку
      (Variables|Default|SethoveredGrid (CallFunction|GetHoveredGrid (Variables|Default|GetGrids)))
      ;[1 1 1] Задаем тайл активной сетки
      (Variables|Default|SethoveredTileOfHoveredGrid _index)
      ;[1 1 1] Добавляем статус для выбранного тайла
      (Default|AddGridTileState (Variables|Default|GethoveredGrid) (Variables|Default|GethoveredTileOfHoveredGrid) "NewEnumerator1")
      (if (Default|IsWalkable (Variables|Default|GethoveredGrid) (.type (.Value (Utilities|Map|Find (Variables|/Game/BP/Core/Grid/BP_Grid.BP_Grid_C|GetgridTiles (Variables|Default|GethoveredGrid)) (Variables|Default|GethoveredTileOfHoveredGrid)))))
        (Audio|PlaySound2D "/Engine/VREditor/Sounds/UI/Object_Snaps_To_Grid.Object_Snaps_To_Grid" 0.5 1.0 0.0 0 0)))))

(fn GetHoveredGrid
  (params (ArrayOfGrids :type Array%20of%20BP%20Grid%20Object%20References))
  ;[1 1 1] Перебираем все сетки
  (for (_array_element _array_index) ArrayOfGrids
    (LocalVariables|SetcurGrid _array_element)
    (LocalVariables|Setind _array_index)
    ;[1 1 1] Позиция тайла данной сетки
    (bind _index (Default|GetTileIndexUnderCursor (LocalVariables|GetcurGrid)))
    ;[1 1 1] Если клетка существует
    (if (Default|IsWalkable (LocalVariables|GetcurGrid) (.type (Utilities|Struct|BreakS_TileData (.Value (Utilities|Map|Find (Variables|/Game/BP/Core/Grid/BP_Grid.BP_Grid_C|GetgridTiles (LocalVariables|GetcurGrid)) _index)))))
      ;[1 1 1] Возвращаем активную сетку
      (return (LocalVariables|GetcurGrid))))
  ;[1 1 1] Если ничего не найдено - оставляем то же значение
  (return (Variables|Default|GethoveredGrid)))

(fn SetSelectedActions
  (params (leftClick :type BP%20Action%20Class%20Reference) (rightClick :type BP%20Action%20Class%20Reference))
  (Utilities|FlowControl|Sequence
    (:then_0
      (Utilities|IsValid (Variables|Default|GetSelectedAction_LMB)
        (:Is%20Valid
          (Actor|DestroyActor (Variables|Default|GetSelectedAction_LMB))
          (Variables|Default|SetSelectedAction_LMB 0))
        (:Is%20Not%20Valid
          _))
      (if (Utilities|IsValidClass leftClick)
        (bind _returnvalue (Game|SpawnActorfromClass leftClick (Math|Transform|MakeTransform "0, 0, 0" "0, 0, 0" "1.000000,1.000000,1.000000") "AlwaysSpawn" 0 self 0))
        (Variables|Default|SetSelectedAction_LMB _returnvalue)))
    (:then_1
      (Utilities|IsValid (Variables|Default|GetSelectedAction_RMB)
        (:Is%20Valid
          (Actor|DestroyActor (Variables|Default|GetSelectedAction_RMB))
          (Variables|Default|SetSelectedAction_RMB 0))
        (:Is%20Not%20Valid
          _))
      (if (Utilities|IsValidClass rightClick)
        (bind _returnvalue_2 (Game|SpawnActorfromClass rightClick (Math|Transform|MakeTransform "0, 0, 0" "0, 0, 0" "1.000000,1.000000,1.000000") "AlwaysSpawn" 0 self 0))
        (Variables|Default|SetSelectedAction_RMB _returnvalue_2)))))

(fn CursoronSelectedGrid
  (return (== (Variables|Default|GetselectedGrid) (Variables|Default|GethoveredGrid))))

(fn UpdateUnitUndertheCursor
  (bind _asbp_charlie_simple (Utilities|Casting|CastToBP_CharlieSimple (.HitActor (Collision|BreakHitResult (.HitResult (Game|Player|GetHitResultUnderCursorbyChannel (Game|GetPlayerController 0) "TraceTypeQuery5" true)))))
    (:then
      (bind _output_get (Variables|Default|SethoveredUnit _asbp_charlie_simple))
      (Variables|/Game/BP/Core/char/BP_CharlieSimple.BP_CharlieSimple_C|SetUIState _output_get "NewEnumerator1")
      (Default|UpdateMaterial _output_get))
    (:CastFailed
      (Utilities|IsValid (Variables|Default|GethoveredUnit)
        (:Is%20Valid
          (Variables|/Game/BP/Core/char/BP_CharlieSimple.BP_CharlieSimple_C|SetUIState (Variables|Default|GethoveredUnit) "NewEnumerator2")
          (Default|UpdateMaterial (Variables|Default|GethoveredUnit))
          (Variables|Default|SethoveredUnit 0))))))

(fn ResetHoveredTile
  (Default|RemoveGridTileState (Variables|Default|GethoveredGrid) (Variables|Default|GethoveredTileOfHoveredGrid) "NewEnumerator1")
  (Variables|Default|SethoveredTileOfHoveredGrid (Utilities|Struct|MakeIntPoint -1 -1)))