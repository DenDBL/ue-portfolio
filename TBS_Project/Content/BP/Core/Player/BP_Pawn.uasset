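; BP_Pawn is the player's camera pawn, providing free movement, rotation and zoom through input axes.
; Axis events update target location along the pawn's forward and right vectors, target yaw rotation, and a clamped zoom length.
; Tick smoothly interpolates the actor transform and spring arm length toward those targets, which the construction script seeds from the initial transform and arm length.
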(event EventTick
  (params (DeltaSeconds :type Float%20%28single-precision%29))
  (Variables|/Script/Engine.SpringArmComponent|SetTargetArmLength (Variables|Default|GetSpringArm) (Math|Interpolation|FInterpTo (Variables|/Script/Engine.SpringArmComponent|GetTargetArmLength (Variables|Default|GetSpringArm)) (Variables|Default|GetzoomLength) DeltaSeconds 5.0))
  (Transformation|SetActorLocation (Math|Interpolation|VInterpTo (Transformation|GetActorLocation) (Variables|Default|GetcameraLocation) DeltaSeconds 5.0) false false)
  (Transformation|SetActorRotation (Math|Interpolation|RInterpTo (Transformation|GetActorRotation) (Variables|Default|GetcameraRotation) DeltaSeconds 5.0)))

(event Input|AxisEvents|InputAxisCameraZoom_Axis
  (params (AxisValue :type Float%20%28single-precision%29))
  (Variables|Default|SetzoomLength (Math|Float|Clamp(Float) (+ (* AxisValue -1e+02) (Variables|Default|GetzoomLength)) 0.0 5e+03)))

(event Input|AxisEvents|InputAxisCameraMoveForward_Axis
  (params (AxisValue :type Float%20%28single-precision%29))
  (Variables|Default|SetcameraLocation (+ (* (* AxisValue (Variables|Default|GetcameraMovementSpeed)) (Transformation|GetActorForwardVector)) (Variables|Default|GetcameraLocation))))

(event Input|AxisEvents|InputAxisCameraMoveSideway_Axis
  (params (AxisValue :type Float%20%28single-precision%29))
  (Variables|Default|SetcameraLocation (+ (* (* AxisValue (Variables|Default|GetcameraMovementSpeed)) (Transformation|GetActorRightVector)) (Variables|Default|GetcameraLocation))))

(event Input|AxisEvents|InputAxisCameraRotation_Axis
  (params (AxisValue :type Float%20%28single-precision%29))
  (Variables|Default|SetcameraRotation (Math|Rotator|CombineRotators (Math|Rotator|MakeRotator 0.0 0.0 (* AxisValue (Variables|Default|GetcameraRotationSpeed))) (Variables|Default|GetcameraRotation))))

(fn ConstructionScript
  (Variables|Default|SetzoomLength (Variables|/Script/Engine.SpringArmComponent|GetTargetArmLength (Variables|Default|GetSpringArm)))
  (Variables|Default|SetcameraLocation (Transformation|GetActorLocation))
  (Variables|Default|SetcameraRotation (Transformation|GetActorRotation)))